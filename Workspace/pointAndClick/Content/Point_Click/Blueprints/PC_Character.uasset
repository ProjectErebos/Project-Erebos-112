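; PC_Character is a point-and-click character prototype that samples the world position under the cursor on mouse click.
; A visibility trace supplies X and Z with Y zeroed, and a DoN reset on release gates each press.
; The click prints "allowed" or "forbidden" from GetVectorLenght, whose distance check against MaximumDistance is disconnected from its entry.
; No movement is implemented.
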(event EventBeginPlay)

(event Collision|EventActorBeginOverlap
  (params (OtherActor :type Actor%20Object%20Reference)))

(event EventTick
  (params (DeltaSeconds :type Float%20%28single-precision%29)))

(event Input|ActionEvents|InputActionMouseClick
  (params (Key :type Key%20Structure))
  (:Pressed
    (bind _mouselocation (CallFunction|GetMouseClickPosition))
    (Variables|Default|Setcurrent%20Mouse%20Position _mouselocation)
    (Utilities|FlowControl|DoN 1 :!label _label
      (:Exit
        (bind _isinrange (CallFunction|GetVectorLenght))
        (if _isinrange
          (Development|PrintString "allowed")
          (else
            (Development|PrintString "forbidden"))))))
  (:Released
    (goto _label Reset)))

(fn ConstructionScript)

(fn GetMouseClickPosition
  (bind _returnvalue (Game|GetPlayerController 0))
  (bind _hitresult (Game|Player|GetHitResultUnderCursorbyChannel _returnvalue "TraceTypeQuery1" true))
  (bind _location (Collision|BreakHitResult _hitresult))
  (bind (_x _y _z) (Math|Vector|BreakVector _location))
  (return (Math|Vector|MakeVector _x 0.0 _z)))

(fn GetVectorLenght)