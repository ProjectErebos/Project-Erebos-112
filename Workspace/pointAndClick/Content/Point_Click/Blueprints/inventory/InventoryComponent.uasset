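; Inventory component for a point-and-click game that holds a fixed-size slot array and toggles an inventory window on the player's HUD canvas.
; Non-stackable items go into the first empty slot; stackable items have no add logic here.
; It also records items chosen for crafting or giving away, clears slots after a successful combination, and plays a random negative response sound for failed player actions.
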(event EventBeginPlay
  (CallFunction|PrepareInventory))

(fn OpenInventory
  (Variables|Default|GetInventoryWindow
    (:then)
    (:else
      (bind _returnvalue (UserInterface|CreateWidget "/Game/Point_Click/Blueprints/inventory/Inventory_UI/InventoryWindow.InventoryWindow_C" 0 self))
      (Variables|Default|SetInventoryWindow _returnvalue)
      (bind _aspc_player_controller (Utilities|Casting|CastToPC_PlayerController (Game|GetPlayerController 0))
        (:then
          (bind _returnvalue_2 (Class|CanvasPanel|AddChildtoCanvas (Variables|/Game/Point_Click/Blueprints/inventory/Inventory_UI/HUD.HUD_C|GetHUDCanvas (Variables|/Game/Point_Click/Blueprints/PC_PlayerController.PC_PlayerController_C|GetHudWidget _aspc_player_controller)) (Variables|Default|GetInventoryWindow)))
          (Class|CanvasPanelSlot|SetAutoSize _returnvalue_2 true)
          (Class|CanvasPanelSlot|SetAlignment _returnvalue_2 "(X=1.000000,Y=1.000000)")
          (Class|CanvasPanelSlot|SetAnchors _returnvalue_2 (Variables|Default|GetAnchors))
          (Input|SetInputModeGameandUI (Game|GetPlayerController 0) (Variables|Default|GetInventoryWindow) "DoNotLock" false)
          (Variables|Default|SetisOpen true))
        (:CastFailed
          (Development|PrintString "Cast has failed"))))))

(fn CloseInventory
  (Variables|Default|GetInventoryWindow
    (:then
      (Widget|RemovefromParent (Variables|Default|GetInventoryWindow))
      (Variables|Default|SetInventoryWindow 0)
      (Variables|Default|SetisOpen false)
      (Input|SetInputModeGameandUI (Game|GetPlayerController 0) 0 "DoNotLock" false))
    (:else)))

(fn AddtoInventory
  (params (addedItem :type Slot%20Structure%20Structure))
  (if (not (.isstackable (.itemstructure addedItem)))
    (CallFunction|CreateStack addedItem)
    (return true)))

(fn PrepareInventory
  (Utilities|Array|Resize (Variables|Default|GetInventory) (Variables|Default|GetnumberOfSlots)))

(fn CreateStack
  (params (ContentToAdd :type Slot%20Structure%20Structure))
  (bind _inventory (Variables|Default|GetInventory))
  (Utilities|Array|SetArrayElem _inventory (Utilities|Array|FindItem _inventory (Utilities|Struct|MakeSlotStructure "(Name_15_21A7EB02419E0AD2686A46A38A2AC814=NSLOCTEXT(\"[9556C5E6472C6A11CB86589A45B81761]\", \"17AC8D6B42B00F0B8C2824B2FD26643C\", \"None\"),isStackable_8_1CA42A4C4107A6CF92DD70A85C11A925=False,Thumbnail_11_06B00CE146E216151320D3A68365D7B4=None,Description_17_B1E31163497FEE62BDFB868C74B5508C=NSLOCTEXT(\"[9556C5E6472C6A11CB86589A45B81761]\", \"F3E7F670423C77456701768BE259ECFE\", \"NotAvailable yet\"),NarraterAudio_45_A3FDAC8541A721C64710EF8FFAC852A3=None,isCombinable_22_19B8A75148DA9E6C54A9E7A360018DC8=False,canBeGivenAway_24_C5E44BB746D2A8F9BEE410BE39310052=False,isConsumable_26_BEFD8B3C4ED6542F70AEE6BF5A0B8B72=False,Permanent_28_7EF8272045EBDFF299C9F7A05EBF52E0=False,MaxStackSize_37_13D876FD478D75760E6F818167C6E814=1,Class_36_D66ACA0E4CE516754FD0CFADED94A575=None,canBeCombinedWith_49_87CF26FA43ABE8C2AE375F9D118AC3E6=None,SuccessfullNarrator_53_78B5E6D644F0D03434C8C69A52F4A240=None,resultingItem_56_B98C5E284CEAAFA4C9A8649097C4A5FD=None)")) ContentToAdd))

(fn BeginCrafting
  (params (firstItemClass :type Item%20Class%20Reference))
  (Variables|Default|SetfirstItemToCraft firstItemClass))

(fn BeginGivingAway
  (params (ItemClassToGive :type Item%20Class%20Reference))
  (Variables|Default|SettoBeGivenAway ItemClassToGive)
  ;[1 1 1] carefulll check if given away correctly
  (return true))

(fn UnsuccessfulPlayer
  (bind _returnvalue (Math|Random|RandomInteger 5))
  (bind _negativeresponce (Variables|Default|GetnegativeResponce))
  (bind _output (Utilities|Array|Get(acopy) _negativeresponce _returnvalue))
  (Audio|PlaySound2D _output _output 1.0 1.0 0.0 0 0))

(fn SuccessfulCombination
  (params (secondSlot :type Integer))
  (bind _slotstructure (Utilities|Struct|MakeSlotStructure "(Name_15_21A7EB02419E0AD2686A46A38A2AC814=NSLOCTEXT(\"[9556C5E6472C6A11CB86589A45B81761]\", \"17AC8D6B42B00F0B8C2824B2FD26643C\", \"None\"),isStackable_8_1CA42A4C4107A6CF92DD70A85C11A925=False,Thumbnail_11_06B00CE146E216151320D3A68365D7B4=None,Description_17_B1E31163497FEE62BDFB868C74B5508C=NSLOCTEXT(\"[9556C5E6472C6A11CB86589A45B81761]\", \"F3E7F670423C77456701768BE259ECFE\", \"NotAvailable yet\"),NarraterAudio_45_A3FDAC8541A721C64710EF8FFAC852A3=None,isCombinable_22_19B8A75148DA9E6C54A9E7A360018DC8=False,canBeGivenAway_24_C5E44BB746D2A8F9BEE410BE39310052=False,isConsumable_26_BEFD8B3C4ED6542F70AEE6BF5A0B8B72=False,Permanent_28_7EF8272045EBDFF299C9F7A05EBF52E0=False,MaxStackSize_37_13D876FD478D75760E6F818167C6E814=1,Class_36_D66ACA0E4CE516754FD0CFADED94A575=None,canBeCombinedWith_49_87CF26FA43ABE8C2AE375F9D118AC3E6=None,SuccessfullNarrator_53_78B5E6D644F0D03434C8C69A52F4A240=None,resultingItem_56_B98C5E284CEAAFA4C9A8649097C4A5FD=None)"))
  (bind _inventory (Variables|Default|GetInventory))
  (Utilities|Array|SetArrayElem _inventory 0 _slotstructure)
  (Utilities|Array|SetArrayElem _inventory secondSlot _slotstructure))